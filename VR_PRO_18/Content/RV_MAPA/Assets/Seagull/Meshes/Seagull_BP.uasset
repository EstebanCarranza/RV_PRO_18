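; Seagull actor that loops a flying animation and emits squawks at random intervals as ambient life.
; BeginPlay starts the looping animation on the skeletal mesh, and plays then immediately stops the Graznidochidillo audio component.
; Tick keeps that component stopped and feeds a random-length Delay, which repeatedly fires the gull cue as non-spatialized 2D sound.
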(event EventBeginPlay
  (bind _graznidochidillo (Variables|Default|GetGraznidochidillo))
  (Audio|Components|Audio|Play _graznidochidillo 0.0)
  (Audio|Components|Audio|Stop _graznidochidillo)
  (Components|Animation|PlayAnimation (Variables|Default|GetSkeletalMesh) "/Game/RV_MAPA/Assets/Seagull/Animations/ANIM_Seagull_Fly.ANIM_Seagull_Fly" true))

(event Collision|EventActorBeginOverlap
  (params (OtherActor :type Actor%20Object%20Reference)))

(event EventTick
  (params (DeltaSeconds :type Float%20%28single-precision%29))
  (Audio|Components|Audio|Stop (Variables|Default|GetGraznidochidillo))
  (Utilities|FlowControl|Delay (Math|Random|RandomFloatinRange 0.1 1e+01))
  (Audio|PlaySound2D "/Game/RV_MAPA/SFX/Gaviota_Cue.Gaviota_Cue"))

(fn ConstructionScript)